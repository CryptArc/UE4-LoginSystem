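; Game Instance Blueprint that handles user login against a PHP web endpoint over HTTP.
; LoginSystem sends the username and password from the Data array as form fields in a URL-encoded POST to SQLRequestURL.
; It caches the username and clears Data so the password is not kept in memory.
; The bound Response event treats an echoed username as success and prints the result on screen.
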(event Custom|LoginSystem
  (bind _data (Variables|Player|Data|GetData))
  (bind _output (Utilities|Array|Get(acopy) _data))
  (bind _output_get (Variables|LoginSystem|SetSQL_Request (Class|VaRestRequestJSON|ConstructRequestExt "POST" "x_www_form_urlencoded_url")))
  (bind _returnvalue (Class|VaRestRequestJSON|GetRequestObject _output_get))
  (Variables|LoginSystem|SetSQL_Request_Object _returnvalue)
  ;[1 1 1] Setting vriables for PHP
  (Class|VaRestJsonObject|SetStringField (Variables|LoginSystem|GetSQL_Request_Object) "username" _output) ; Create $_REQUEST['username'];
  (Variables|Player|Data|SetData_Username _output) ; We will delete later this array. We need to keep the username
  (Class|VaRestJsonObject|SetStringField (Variables|LoginSystem|GetSQL_Request_Object) "password" (Utilities|Array|Get(acopy) (Variables|Player|Data|GetData) 1)) ; Create $_REQUEST['password'];
  ;[1 1 1] Send Request (variables) to the URL
  (Class|VaRestRequestJSON|ProcessURL (Variables|LoginSystem|GetSQL_Request) (Variables|LoginSystem|GetSQL_Request_URL))
  (EventDispatchers|BindEventtoOnRequestComplete (Variables|LoginSystem|GetSQL_Request) (delegate Custom|Response))
  ;[1 1 1] Dump the Data array, we don't want to keep the password ingame the whole time.
  (Utilities|Array|Clear (Variables|Player|Data|GetData)))

(event Custom|Response
  (params (Request :type Va%20Rest%20Request%20JSON%20Object%20Reference))
  (if (Utilities|Enum|Equal(Enum) (Variables|/Script/VaRestPlugin.VaRestRequestJSON|GetResponseContent Request) (Variables|Player|Data|GetData_Username))
    (Development|PrintString "Logged in" true true "(R=0.000000,G=0.660000,B=1.000000,A=1.000000)" 1e+01)
    (else
      (Development|PrintString "Login Failed" true true "(R=0.000000,G=0.660000,B=1.000000,A=1.000000)" 1e+01))))